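; Base tower for a tower defense game that automatically attacks enemies entering its detection radius.
; Overlap events track enemies in range, and a self-rescheduling timer deals damage at a rate set by attack speed.
; When no target is found, the attack is buffered and fires as soon as an enemy enters the empty range.
; A priority setting picks the target by furthest path progress, least path progress, or highest level.
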(event OnComponentBeginOverlap(DetectionRadius)
  (params (OverlappedComponent :type Primitive%20Component%20Object%20Reference) (OtherActor :type Actor%20Object%20Reference) (OtherComp :type Primitive%20Component%20Object%20Reference) (OtherBodyIndex :type Integer) (bFromSweep :type Boolean) (SweepResult :type Hit%20Result%20Structure%20%28by%20ref%29))
  (bind _enemiesinrange (Variables|Default|GetEnemiesInRange))
  (bind _asenemy_base (Utilities|Casting|CastToEnemyBase OtherActor))
  (Utilities|Array|AddUnique _enemiesinrange _asenemy_base)
  (if (== (Utilities|Array|Length _enemiesinrange) 1)
    (if (Variables|Default|GetBuffer%20Attack)
      (CallFunction|Attack))))

(event OnComponentEndOverlap(DetectionRadius)
  (params (OverlappedComponent :type Primitive%20Component%20Object%20Reference) (OtherActor :type Actor%20Object%20Reference) (OtherComp :type Primitive%20Component%20Object%20Reference) (OtherBodyIndex :type Integer))
  (bind _enemiesinrange (Variables|Default|GetEnemiesInRange))
  (bind _asenemy_base (Utilities|Casting|CastToEnemyBase OtherActor))
  (if (Utilities|Array|ContainsItem _enemiesinrange _asenemy_base)
    (Utilities|Array|RemoveItem _enemiesinrange _asenemy_base)))

(event Custom|Attack
  (bind _target (CallFunction|GetTarget))
  (Utilities|IsValid _target
    (:Is%20Valid
      (CallFunction|DealDamage _target)
      (Variables|Default|SetBuffer%20Attack false)
      (Utilities|Time|SetTimerbyEvent (delegate Custom|Attack) (CallFunction|ComputeAttackInterval)))
    (:Is%20Not%20Valid
      (Variables|Default|SetBuffer%20Attack true))))

(event Custom|Deal%20Damage
  (params (Target :type Enemy%20Base%20Object%20Reference))
  (Default|TakeDamage Target 1))

(event EventBeginPlay
  (bind _returnvalue (Rendering|Material|CreateDynamicMaterialInstance "/Game/Art/Materials/EnemyMaterial.EnemyMaterial" "None" :!class /Script/Engine.KismetMaterialLibrary))
  (bind _output_get (Variables|Default|SetSpriteMaterial _returnvalue))
  (Rendering|Material|SetMaterial (Variables|Default|GetPaperSprite) 0 _output_get))

(fn ConstructionScript)

(fn ComputeAttackInterval
  (return (/ 1.0 (Variables|Default|GetAttack%20Speed%20Base))))

(fn GetTarget
  (switch Utilities|FlowControl|Switch|SwitchonTargetPriority (Variables|Default|GetTargetPriority)
    (:NewEnumerator0
      (bind _first_enemy (CallFunction|GetFirstTarget))
      (return _first_enemy))
    (:NewEnumerator1
      (bind _strongest_enemy (CallFunction|GetStrongTarget))
      (return _strongest_enemy))
    (:NewEnumerator2
      (bind _last_enemy (CallFunction|GetLastTarget))
      (return _last_enemy))))

(fn GetFirstTarget
  (for _array_element (Variables|Default|GetEnemiesInRange)
    (Utilities|IsValid (LocalVariables|GetFirst)
      (:Is%20Valid
        (if (> (Default|GetPathAlpha _array_element) (LocalVariables|GetBestDistance))
          (bind _output_get (LocalVariables|SetFirst _array_element :!label _label))
          (LocalVariables|SetBestDistance (Default|GetPathAlpha _output_get))))
      (:Is%20Not%20Valid
        (goto _label))))
  (return (LocalVariables|GetFirst)))

(fn GetStrongTarget
  (for _array_element (Variables|Default|GetEnemiesInRange)
    (Utilities|IsValid (LocalVariables|GetStrong)
      (:Is%20Valid
        (if (> (Variables|/Game/Blueprints/EnemyBase.EnemyBase_C|GetLevel _array_element) (LocalVariables|GetBestLevel))
          (bind _output_get (LocalVariables|SetStrong _array_element :!label _label))
          (LocalVariables|SetBestLevel (Variables|/Game/Blueprints/EnemyBase.EnemyBase_C|GetLevel _output_get))))
      (:Is%20Not%20Valid
        (goto _label))))
  (return (LocalVariables|GetStrong)))

(fn GetLastTarget
  (for _array_element (Variables|Default|GetEnemiesInRange)
    (Utilities|IsValid (LocalVariables|GetLast)
      (:Is%20Valid
        (if (< (Default|GetPathAlpha _array_element) (LocalVariables|GetBestDistance))
          (bind _output_get (LocalVariables|SetLast _array_element :!label _label))
          (LocalVariables|SetBestDistance (Default|GetPathAlpha _output_get))))
      (:Is%20Not%20Valid
        (goto _label))))
  (return (LocalVariables|GetLast)))