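; Item Blueprint that derives its name from a primary and secondary particle category: Electron, Photon, Graviton or Neutrino.
; GetItemName sorts the two enum values with byte min/max, so category order does not matter.
; The lower value selects the prefix and the higher the suffix, joined without a space; None yields an empty string.
; Event graph and construction script are empty, and the Neutrino suffix is a "????" placeholder.
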(event EventBeginPlay)

(event Collision|EventActorBeginOverlap
  (params (OtherActor :type Actor%20Object%20Reference)))

(event EventTick
  (params (DeltaSeconds :type Float%20%28single-precision%29)))

(fn ConstructionScript)

(fn GetItemName
  (bind _primary_category (Variables|Default|GetPrimary%20Category))
  (bind _secondary_category (Variables|Default|GetSecondary%20Category))
  (return (Utilities|String|StringToName (Utilities|String|Append (Utilities|Select :Index (Utilities|Enum|ByteToEnumItemCategory (Class|KismetMathLibrary|BMin _primary_category _secondary_category)) :NewEnumerator4 "" :NewEnumerator0 "Electron" :NewEnumerator1 "Photon" :NewEnumerator2 "Graviton" :NewEnumerator3 "Neutrino") (Utilities|Select :Index (Utilities|Enum|ByteToEnumItemCategory (Class|KismetMathLibrary|BMax _primary_category _secondary_category)) :NewEnumerator4 "" :NewEnumerator0 "Conductor" :NewEnumerator1 "Beam" :NewEnumerator2 "Accelerator" :NewEnumerator3 "????")))))