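; Tower placement preview actor that follows the mouse cursor, showing the tower to be placed via a ChildActor.
; Each tick it checks the tower's PlacementCollision for overlaps and tints its sprite white or red when placement validity changes, based on overlap and the player's money.
; Drop spawns a real tower of that class, starts its attack, deducts the cost from the game state and destroys the preview.
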(event EventBeginPlay
  (CallFunction|UpdateTowerStatus true))

(event EventTick
  (params (DeltaSeconds :type Float%20%28single-precision%29))
  (bind _can_drop (CallFunction|CanDrop))
  (Utilities|FlowControl|Sequence
    (:then_0
      (bind _location (Default|GetMouseWorldLocation (.AsSubatomic%20Player%20Controller (Utilities|Casting|CastToSubatomicPlayerController (Game|GetPlayerController 0)))))
      (Transformation|SetActorLocation (+ _location "0, 0,5.000000") false false))
    (:then_1
      (Variables|Default|SetOverlapping (> (Utilities|Array|Length (Collision|GetOverlappingActors (Variables|/Game/Blueprints/TowerBase.TowerBase_C|GetPlacementCollision (.AsTower%20Base (Utilities|Casting|CastToTowerBase (Variables|/Script/Engine.ChildActorComponent|GetChildActor (Variables|Default|GetChildActor))))) 0 :!class /Script/Engine.PrimitiveComponent)) 0)))
    (:then_2
      (if (Math|Boolean|NotEqual(Boolean) (Variables|Default|GetPreviousDroppable) _can_drop)
        (CallFunction|UpdateTowerStatus _can_drop))
      (Variables|Default|SetPreviousDroppable _can_drop))))

(fn ConstructionScript)

(fn Drop
  (if (CallFunction|CanDrop)
    (bind _returnvalue (Game|SpawnActorfromClass (Variables|/Script/Engine.ChildActorComponent|GetChildActorClass (Variables|Default|GetChildActor)) (Transformation|GetActorTransform) "AlwaysSpawn" 0 0))
    (Default|Attack (.AsTower%20Base (Utilities|Casting|CastToTowerBase _returnvalue)))
    (Default|ModifyMoney (.AsSubatomic%20Game%20State (Utilities|Casting|CastToSubatomicGameState (Game|GetGameState))) (* (Variables|/Game/Blueprints/TowerBase.TowerBase_C|GetCost (.AsTower%20Base (Utilities|Casting|CastToTowerBase (Variables|/Script/Engine.ChildActorComponent|GetChildActor (Variables|Default|GetChildActor))))) -1))
    (Actor|DestroyActor)
    (return true)
    (else
      (return false))))

(fn CanDrop
  (return (and (>= (Variables|/Game/Blueprints/GameRelated/SubatomicGameState.SubatomicGameState_C|GetMoney (.AsSubatomic%20Game%20State (Utilities|Casting|CastToSubatomicGameState (Game|GetGameState)))) (Variables|/Game/Blueprints/TowerBase.TowerBase_C|GetCost (.AsTower%20Base (Utilities|Casting|CastToTowerBase (Variables|/Script/Engine.ChildActorComponent|GetChildActor (Variables|Default|GetChildActor)))))) (not (Variables|Default|GetOverlapping)))))

(fn UpdateTowerStatus
  (params (Valid :type Boolean))
  (Rendering|Material|SetVectorParameterValue (Variables|/Game/Blueprints/TowerBase.TowerBase_C|GetSpriteMaterial (.AsTower%20Base (Utilities|Casting|CastToTowerBase (Variables|/Script/Engine.ChildActorComponent|GetChildActor (Variables|Default|GetChildActor))))) "Tint" (Math|Color|SelectColor "(R=1.000000,G=1.000000,B=1.000000,A=1.000000)" "(R=1.000000,G=0.000000,B=0.000000,A=1.000000)" Valid) :!class /Script/Engine.MaterialInstanceDynamic))