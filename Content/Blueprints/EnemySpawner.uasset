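; Enemy spawner that works through a list of spawn definitions from BeginPlay, creating timed runs of EnemyBase actors.
; SpawnEnemy decrements the current entry's repetitions, spawns an enemy at the world origin with that entry's path index and level, then re-arms itself by timer after the entry's delay.
; An exhausted entry advances the index and recurses immediately, and spawning stops at the end of the list.
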(event Custom|Spawn%20Enemy
  (bind _spawnlist (Variables|Default|GetSpawnList))
  (bind _index (Variables|Default|GetIndex))
  (bind _output (Utilities|Array|Get(acopy) _spawnlist _index))
  (bind (_level _delay _path _repetitions) (Utilities|Struct|BreakEnemySpawnDefinition _output))
  (if (< (Variables|Default|GetIndex) (Utilities|Array|Length (Variables|Default|GetSpawnList)))
    (if (> _repetitions 0)
      (Utilities|Struct|SetmembersinEnemySpawnDefinition _output (- _repetitions 1))
      (Game|SpawnActorfromClass "/Game/Blueprints/EnemyBase.EnemyBase_C" (Math|Transform|MakeTransform "0, 0, 0") "Undefined" 0 _path _level 0)
      (Utilities|Time|SetTimerbyEvent (delegate Custom|Spawn%20Enemy) _delay)
      (else
        (Math|Integer|IncrementInt (Variables|Default|GetIndex)
          (:%20%20
            (CallFunction|SpawnEnemy)))))))

(event EventBeginPlay
  (CallFunction|SpawnEnemy))

(fn ConstructionScript)