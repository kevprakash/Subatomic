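; Base tower-defense enemy actor that follows a spline Path and, on reaching the end, damages SubatomicGameState by its Level.
; BeginPlay finds the Path matching PathIndex if none is set, applies the Level, then plays the Movement timeline, which drives position and spin.
; Level doubles as health, selecting sprite and speed, with play rate normalized by spline length.
; Damage drops the Level or destroys the enemy.
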(event Custom|Set%20Level
  (params (Level :type Integer))
  (bind _output_get (Variables|Default|SetLevel Level))
  (bind _output_get_2 (Variables|Default|SetRelativeSpeed (/ (.Value (Utilities|Map|Find (Variables|Default|GetSpeed) _output_get)) (Spline|GetSplineLength (Variables|/Game/Blueprints/Path.Path_C|GetSpline (Variables|Default|GetPathToFollow))))))
  (Components|Timeline|SetPlayRate (Variables|Default|GetMovement) _output_get_2)
  (Rendering|Components|Sprite|SetSprite (Variables|Default|GetPaperSprite) (.Value (Utilities|Map|Find (Variables|Default|GetSprite) (Variables|Default|GetLevel)))))

(event Custom|Take%20Damage
  (params (Amount :type Integer))
  (bind _level (Variables|Default|GetLevel))
  (if (>= Amount _level)
    (CallFunction|OnDeath)
    (else
      (CallFunction|SetLevel (- _level Amount)))))

(event Custom|OnDeath
  (Actor|DestroyActor))

(event EventBeginPlay
  (Utilities|FlowControl|Sequence
    (:then_0
      (Utilities|IsValid (Variables|Default|GetPathToFollow)
        (:Is%20Not%20Valid
          (bind _outactors (Actor|GetAllActorsOfClass "/Game/Blueprints/Path.Path_C"))
          (bind _array_element (Utilities|Array|ForEachLoopwithBreak _outactors :!label _label)
            (:LoopBody
              (if (== (Variables|/Game/Blueprints/Path.Path_C|GetIndex _array_element) (Variables|Default|GetPath%20Index))
                (Variables|Default|SetPathToFollow _array_element)
                (goto _label Break)))))))
    (:then_1
      (CallFunction|SetLevel (Variables|Default|GetLevel)))
    (:then_2
      (Components|Timeline|PlayfromStart (Variables|Default|GetMovement)))))

(fn ConstructionScript)

(fn GetPathAlpha
  (return (Components|Timeline|GetPlaybackPosition (Variables|Default|GetMovement))))