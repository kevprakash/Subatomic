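; Player controller that shows the mouse cursor and turns the Click input into a tower placement.
; On click, PlaceTower finds a Dropper actor in the level and, if valid, calls its Drop function.
; GetMouseWorldLocation deprojects the cursor and line traces into the world to return the hit location, though nothing in this Blueprint calls it.
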(event EventBeginPlay
  (Variables|Default|SetbShowMouseCursor true))

(event EventTick
  (params (DeltaSeconds :type Float%20%28single-precision%29)))

(event Input|ActionEvents|InputActionClick
  (params (Key :type Key%20Structure))
  (:Pressed
    (CallFunction|PlaceTower)))

(fn ConstructionScript)

(fn GetMouseWorldLocation
  (bind (_worldlocation _worlddirection) (Game|Player|ConvertMouseLocationToWorldSpace))
  (bind _outhit (Collision|LineTraceByChannel _worldlocation (+ _worldlocation (* _worlddirection 5e+03)) "TraceTypeQuery3" true 0 "None"))
  (return (.location _outhit)))

(fn PlaceTower
  (bind _returnvalue (Actor|GetActorOfClass "/Game/Blueprints/Dropper.Dropper_C"))
  (Utilities|IsValid _returnvalue
    (:Is%20Valid
      (Default|Drop _returnvalue))))